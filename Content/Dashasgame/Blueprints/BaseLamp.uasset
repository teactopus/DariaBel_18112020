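; BaseLamp is a lamp Blueprint that switches its PointLight between a set intensity and zero.
; BeginPlay applies the Onoff state, then shares the Repeat event's two-second delay before a single inverted SwitchLight call, with no loop back.
; SwitchLight ignores its input and sets Onoff to false before branching, so the light always ends at zero intensity.
; Tick, the construction script and the test functions are placeholders.
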(event `Repeat`
  ;[1 1 1] вызов логики с задержкой
  (`KismetSystemLibrary.Delay` 2.0 :!label _label)
  (`self.switch light` (not (`self.On/off`))))

(event `self.ReceiveTick`
  (params (DeltaSeconds :type "Float (single-precision)"))
  ;[1 1 1] вызывается раз в 60 секунд
)

(event `self.ReceiveBeginPlay`
  (`self.switch light` (`self.On/off`))
  (goto _label))

(fn `my test function`
  (params (` TestBool` :type Boolean) (InString :type String))
  (returns (NewParam1 :type Boolean))
  (return false))

(fn `NewFunction_0`)

(fn `switch light`
  (params (`On/Off` :type Boolean))
  (set `self.On/off` false)
  (if (`self.On/off`)
    (`LightComponent.SetIntensity` (`self.PointLight`) (`self.MiIntencity`))
    (else
      (`LightComponent.SetIntensity` (`self.PointLight`) 0.0))))

(fn `UserConstructionScript`)